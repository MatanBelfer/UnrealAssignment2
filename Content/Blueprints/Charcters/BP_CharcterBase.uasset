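; BP_CharcterBase is a base character Blueprint that handles health, damage and death.
; Health starts at MaxHealth, and ReciveDamage subtracts damage, then either calls UpdateUIEvent or, at zero or below, clamps Health and calls Die.
; Die disables input, reports the character to BP_GameMode through OnDied and destroys the actor.
; UpdateUIEvent forwards to UpdateUI, which is empty here and is skipped on a lethal hit.
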(event Custom|UpdateUIEvent
  (CallFunction|UpdateUI))

(event EventBeginPlay
  (Variables|Default|SetHealth (Variables|Default|GetMaxHealth)))

(event Collision|EventActorBeginOverlap
  (params (OtherActor :type Actor%20Object%20Reference)))

(event EventTick
  (params (DeltaSeconds :type Float%20%28single-precision%29)))

(event EventReciveDamage
  (params (Damage :type Float%20%28double-precision%29) (DamageInstigator :type Actor%20Object%20Reference))
  (if (<= (- (Variables|Default|GetHealth) Damage) 0.0)
    (Variables|Default|SetHealth 0.0)
    (CallFunction|Die)
    (else
      (Variables|Default|SetHealth (- (Variables|Default|GetHealth) Damage))
      (CallFunction|UpdateUIEvent))))

(event EventDie
  (Input|DisableInput 0)
  (bind _asbp_game_mode (Utilities|Casting|CastToBP_GameMode (Game|GetGameMode)))
  (Default|OnDied _asbp_game_mode self)
  (Actor|DestroyActor))

(fn ConstructionScript)

(fn UpdateUI)