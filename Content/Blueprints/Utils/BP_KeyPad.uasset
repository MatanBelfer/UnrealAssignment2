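; Keypad actor that checks an entered code and opens an attached item when it matches.
; Ten BP_Key child actors are labelled by array index in the construction script, then numbered and bound to a press event on BeginPlay.
; Presses append digits to the displayed input until it reaches code length.
; A match plays sounds and a timeline lerping OpenItem to EndTransform; a mismatch clears the input and resets the keys.
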(event Custom|OnButtonPressed_Event
  (params (number :type Integer))
  (bind _output_get (Variables|Default|SetCurrentInput (Utilities|String|Append (Variables|Default|GetCurrentInput) (Utilities|String|ToString(Integer) number))))
  (Rendering|Components|TextRender|SetText (Variables|Default|GetTextRender) (Utilities|Text|ToText(String) _output_get))
  (if (>= (Utilities|String|Len _output_get) (Utilities|String|Len (Variables|Default|GetCode)))
    (if (Utilities|Enum|Equal(Enum) (Variables|Default|GetCurrentInput) (Variables|Default|GetCode))
      (Audio|PlaySoundatLocation "/Engine/VREditor/Sounds/VR_open.VR_open" (Transformation|GetWorldLocation (Variables|Default|GetKeypad_Base)) "0, 0, 0" 1.0 1.0 0.0 0 0 0 0)
      (Audio|PlaySoundatLocation "/Game/sound/3D_PRESSH.3D_PRESSH" (Transformation|GetWorldLocation (Variables|Default|GetOpen_Item)) "0, 0, 0" 1.0 1.0 0.0 0 0 0 0)
      (bind _openup (Timeline|TL_Open_Item Play)
        (:Update
          (Transformation|SetRelativeTransform (Variables|Default|GetOpen_Item) (Math|Transform|Lerp(Transform) (Variables|Default|GetStartTransform) (Variables|Default|GetEndTransform) _openup) false false)))
      (else
        (Variables|Default|SetCurrentInput "")
        (for _array_element (Variables|Default|GetKeysArray)
          (bind _asbp_key (Utilities|Casting|CastToBP_Key (Variables|/Script/Engine.ChildActorComponent|GetChildActor _array_element)))
          (Default|Reset _asbp_key))))
    (else
      (Development|PrintString (Variables|Default|GetCurrentInput)))))

(event EventBeginPlay
  (Variables|Default|SetStartTransform (Transformation|GetRelativeTransform (Variables|Default|GetOpen_Item)))
  (for _array_element (Variables|Default|GetKeysArray)
    (bind _asbp_key (Utilities|Casting|CastToBP_Key (Variables|/Script/Engine.ChildActorComponent|GetChildActor _array_element)))
    (EventDispatchers|BindEventtoOnButtonPressed _asbp_key (delegate Custom|OnButtonPressed_Event))
    (bind (_array_element_2 _array_index) (Utilities|Array|ForEachLoopwithBreak (Variables|Default|GetKeysArray))
      (:LoopBody
        (bind _asbp_key_2 (Utilities|Casting|CastToBP_Key (Variables|/Script/Engine.ChildActorComponent|GetChildActor _array_element_2)))
        (Default|SetNumber _asbp_key_2 _array_index)))))

(fn ConstructionScript
  (bind _output_get (Variables|Default|SetKeysArray (Utilities|Array|MakeArray (Variables|Default|GetBP_Key0) (Variables|Default|GetBP_Key1) (Variables|Default|GetBP_Key2) (Variables|Default|GetBP_Key3) (Variables|Default|GetBP_Key4) (Variables|Default|GetBP_Key5) (Variables|Default|GetBP_Key6) (Variables|Default|GetBP_Key7) (Variables|Default|GetBP_Key8) (Variables|Default|GetBP_Key9))))
  (bind (_array_element _array_index) (Utilities|Array|ForEachLoopwithBreak _output_get)
    (:LoopBody
      (bind _asbp_key (Utilities|Casting|CastToBP_Key (Variables|/Script/Engine.ChildActorComponent|GetChildActor _array_element)))
      (Rendering|Components|TextRender|SetText (Variables|/Game/Blueprints/Utils/BP_Key.BP_Key_C|GetTXT_BTN _asbp_key) (Utilities|Text|ToText(Integer) _array_index)))))