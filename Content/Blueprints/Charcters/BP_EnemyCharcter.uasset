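; Enemy character with an Idle, Patrol and Chase state machine that hunts and attacks the player.
; Patrol walks looping waypoints, pausing in Idle at each, while range, FOV dot-product and line-trace checks scan for the player.
; A clear sighting runs down an aggro timer into Chase, which pursues, attacks on cooldown and de-aggros after losing the view cone.
; State changes update the anim instance; UpdateUI sets the health bar.
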(event Custom|ChaseMoveTo_Event
  (AI|AIMoveTo self (Transformation|GetActorLocation (Variables|Default|GetPlayer)) 0 5e+01 true))

(event Custom|Attack
  (params (Damage :type Float%20%28double-precision%29) (AttackTarget :type BP%20Charcter%20Base%20Object%20Reference))
  (Default|ReciveDamage AttackTarget Damage self)
  (Utilities|FlowControl|Delay 5.0)
  (Variables|Default|SetIsAttacking false))

(event Custom|PatrolMoveTo_Event
  (bind _patrolpoints (Variables|Default|GetPatrolPoints))
  (if (not (Variables|Default|GetIsWalkingToPoint))
    (if (> (Utilities|Array|Length _patrolpoints) 0)
      (Variables|Default|SetIsWalkingToPoint true)
      (AI|AIMoveTo self (Transformation|GetWorldLocation (Variables|/Script/Engine.Actor|GetRootComponent (Utilities|Array|Get(acopy) _patrolpoints (Variables|Default|GetCurrentPointIndex)))) 0 5.0 false
        (:OnSuccess
          (StateCore|ChangeState "NewEnumerator0")
          (Utilities|FlowControl|Delay 5.0)
          (Variables|Default|SetIsWalkingToPoint false)
          (bind _result (Math|Integer|IncrementInt (Variables|Default|GetCurrentPointIndex))
            (:%20%20
              (bind _output_get (Variables|Default|SetCurrentPointIndex _result))
              (if (== _output_get (Utilities|Array|Length (Variables|Default|GetPatrolPoints)))
                (Variables|Default|SetCurrentPointIndex 0)))))))))

(event EventBeginPlay
  (|CallParentFunction)
  (Variables|Default|SetStartTransform (Transformation|GetActorTransform))
  (bind _asbp_player_character (Utilities|Casting|CastToBP_PlayerCharacter (Game|GetPlayerCharacter 0)))
  (Variables|Default|SetPlayer _asbp_player_character)
  (CallFunction|UpdateUI)
  (Variables|/Script/Engine.CharacterMovementComponent|SetMaxWalkSpeed (Variables|Character|GetCharacterMovement) (Variables|Default|GetMax%20Walk%20Speed)))

(event EventTick
  (params (DeltaSeconds :type Float%20%28single-precision%29))
  (switch Utilities|FlowControl|Switch|SwitchonEnemyStates (Variables|Default|GetCurrentState)
    (:NewEnumerator0
      (IdleState|IdleTickState))
    (:NewEnumerator1
      (PatrolState|PatrolTickState))
    (:NewEnumerator2
      (ChaseState|ChaseTickState))))

(fn ConstructionScript
  (|CallParentFunction))

(fn ChangeState
  (params (NewState :type EnemyStates%20Enum :default "NewEnumerator0"))
  (if (Utilities|Enum|Equal(Enum) NewState (Variables|Default|GetCurrentState))
    (if (Variables|Default|GetIsInitialState)
      (Variables|Default|SetIsInitialState false)
      (switch Utilities|FlowControl|Switch|SwitchonEnemyStates (Variables|Default|GetCurrentState) :!label _label
        (:NewEnumerator0
          (IdleState|IdleExitState))
        (:NewEnumerator1
          (PatrolState|PatrolExitState))
        (:NewEnumerator2
          (ChaseState|ChaseExitState)))
      (bind _output_get (Variables|Default|SetCurrentState NewState))
      (switch Utilities|FlowControl|Switch|SwitchonEnemyStates _output_get
        (:NewEnumerator0
          (IdleState|IdleEnterState))
        (:NewEnumerator1
          (PatrolState|PatrolEnterState))
        (:NewEnumerator2
          (ChaseState|ChaseEnterState)))
      (Development|PrintString (Utilities|String|Append "enter state :" (Utilities|String|EnumtoString _output_get)))
      (bind _asbpa_enemy (Utilities|Casting|CastToBPA_Enemy (Components|SkeletalMesh|GetAnimInstance (Variables|Character|GetMesh))))
      (Default|SetState _asbpa_enemy _output_get)
      (else
        (Development|PrintString "changing from current state to same state ")))
    (else
      (goto _label))))

(fn IdleEnterState)

(fn PatrolEnterState)

(fn PatrolTickState
  (bind (_playerfoundouterscoup _playerfoundinnerscoup _playerclearsight) (CallFunction|ScanforPlayer))
  (if (and _playerfoundinnerscoup _playerclearsight)
    (Transformation|SetActorRotation (Math|Rotator|FindLookatRotation (Transformation|GetWorldLocation (Variables|Default|GetEyes)) (Transformation|GetWorldLocation (Variables|/Game/Blueprints/Charcters/BP_PlayerCharacter.BP_PlayerCharacter_C|GetTargetPoint (Variables|Default|GetPlayer)))))
    (bind (_returnvalue _countdownreturn) (CallFunction|Countdown (Variables|Default|GetAggroCountdown)))
    (Variables|Default|SetAggroCountdown _countdownreturn)
    (if _returnvalue
      (StateCore|ChangeState "NewEnumerator2"))
    (else
      (CallFunction|PatrolMovetoEvent)
      (Variables|Default|SetAggroCountdown (Math|Float|Clamp(Float) (+ (Variables|Default|GetAggroCountdown) (Utilities|Time|GetWorldDeltaSeconds)) 0.0 5.0)))))

(fn PatrolExitState
  (Variables|Default|SetAggroCountdown 5.0))

(fn IdleTickState
  (if (not (Variables|Default|GetIsWalkingToPoint))
    (StateCore|ChangeState "NewEnumerator1")))

(fn IdleExitState)

(fn ChaseEnterState)

(fn ChaseTickState
  (bind _playerfoundinnerscoup (CallFunction|ScanforPlayer))
  (if _playerfoundinnerscoup
    (Variables|Default|SetDeAggroCountdown (Math|Float|Clamp(Float) (+ (Variables|Default|GetDeAggroCountdown) (Utilities|Time|GetWorldDeltaSeconds)) 0.0 5.0))
    (if (<= (Transformation|GetDistanceTo self (Variables|Default|GetPlayer)) (LocalVariables|GetAttackRange))
      (if (not (Variables|Default|GetIsAttacking))
        (Variables|Default|SetIsAttacking true)
        (CallFunction|Attack (Variables|Default|GetAttackDamage) (Variables|Default|GetPlayer)))
      (else
        (CallFunction|ChaseMovetoEvent)))
    (else
      (bind (_returnvalue _countdownreturn) (CallFunction|Countdown (Variables|Default|GetDeAggroCountdown)))
      (Variables|Default|SetDeAggroCountdown _countdownreturn)
      (if _returnvalue
        (StateCore|ChangeState "NewEnumerator1")))))

(fn ChaseExitState
  (Variables|Default|SetDeAggroCountdown 5.0))

(fn UpdateUI
  (Development|PrintString (Utilities|String|Append "Current " (Utilities|GetObjectName self) " Health " (Utilities|String|ToString(Float) (Variables|Default|GetHealth))) true true "(R=0.023114,G=1.000000,B=0.169924,A=1.000000)" 5.0)
  (bind _asenemy_health_bar (Utilities|Casting|CastToEnemy_HealthBar (UserInterface|GetWidget (Variables|Default|GetHealthBar))))
  (Progress|SetPercent (Variables|/Game/Blueprints/UI/Enemy_HealthBar.Enemy_HealthBar_C|GetHealthBar _asenemy_health_bar) (/ (Variables|Default|GetHealth) 1e+02)))

(fn ScanforPlayer
  (bind _output_get (LocalVariables|SetPlayerLoc (Transformation|GetWorldLocation (Variables|/Game/Blueprints/Charcters/BP_PlayerCharacter.BP_PlayerCharacter_C|GetTargetPoint (Variables|Default|GetPlayer)))))
  (bind _output_get_2 (LocalVariables|SetSelfLoc (Transformation|GetWorldLocation (Variables|Default|GetEyes))))
  (bind _output_get_3 (LocalVariables|SetToPlayer (- _output_get _output_get_2)))
  (if (<= (Math|Vector|VectorLength _output_get_3) (Variables|Default|GetLoosingSightRange))
    (if (<= (Math|Vector|VectorLength (LocalVariables|GetToPlayer)) (Variables|Default|GetSightRange))
      (bind _output_get_4 (LocalVariables|SetDirToPlayer (Math|Vector|Normalize _output_get_3)))
      (LocalVariables|SetDot (Math|Vector|DotProduct _output_get_4 (Transformation|GetActorForwardVector)))
      (bind _output_get_5 (LocalVariables|SetHalfFOV (* (Variables|Default|GetFOVDegrees) 0.5)))
      (bind _output_get_6 (LocalVariables|SetHalfFOVRadians (Math|Trig|DegreesToRadians _output_get_5)))
      (bind _output_get_7 (LocalVariables|SetDotThreshold (Math|Trig|Cos(Radians) _output_get_6)))
      (if (>= (LocalVariables|GetDot) _output_get_7)
        (bind _outhit (Collision|LineTraceByChannel (Transformation|GetWorldLocation (Variables|Default|GetEyes)) (Transformation|GetWorldLocation (Variables|/Game/Blueprints/Charcters/BP_PlayerCharacter.BP_PlayerCharacter_C|GetTargetPoint (Variables|Default|GetPlayer))) "TraceTypeQuery1" false 0 "Persistent"))
        (return true true (== (Variables|Default|GetPlayer) (.hitactor _outhit)) (LocalVariables|GetDirToPlayer))
        (else
          (return true false false "0, 0, 0"))))
    (else
      (return false false false "0, 0, 0"))))

(fn Countdown
  (params (Countdown :type Float%20%28double-precision%29))
  (bind _output_get (LocalVariables|SetLocalCountdown (- Countdown (Utilities|Time|GetWorldDeltaSeconds))))
  (return (<= _output_get 0.0) _output_get))