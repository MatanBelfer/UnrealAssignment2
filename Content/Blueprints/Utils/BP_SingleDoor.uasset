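; BP_SingleDoor is a sliding door that opens automatically when a character derived from BP_CharcterBase enters its trigger zone.
; The OpenDoor timeline slides the Door component along its relative Y axis.
; When the timeline finishes, a timer, looping while IsOpen is true, calls TryCloseDoor, which reverses the timeline once no actors of any class overlap the zone.
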(event OnComponentBeginOverlap(Trigger_Zone)
  (params (OverlappedComponent :type Primitive%20Component%20Object%20Reference) (OtherActor :type Actor%20Object%20Reference) (OtherComp :type Primitive%20Component%20Object%20Reference) (OtherBodyIndex :type Integer) (bFromSweep :type Boolean) (SweepResult :type Hit%20Result%20Structure%20%28by%20ref%29))
  (if (Utilities|ClassIsChildOf (Utilities|GetClass OtherActor) "/Game/Blueprints/Charcters/BP_CharcterBase.BP_CharcterBase_C")
    (Variables|Default|SetIsOpen true)
    (bind _opendoor (Timeline|OpenDoor Play)
      (:Update
        (Transformation|SetRelativeLocation (Variables|Default|GetDoor) (Math|Vector|MakeVector 0.0 (Math|Float|Lerp 0.0 2.6e+02 _opendoor) 0.0) false false))
      (:Finished
        (Utilities|Time|SetTimerbyEvent (delegate Custom|TryCloseDoor) 1.0 (stale Custom|TryCloseDoor _output_get))))))

(event Custom|TryCloseDoor
  (if (not (> (Utilities|Array|Length (Collision|GetOverlappingActors (Variables|Default|GetTrigger_Zone) 0 :!class /Script/Engine.PrimitiveComponent)) 0))
    (bind _output_get (Variables|Default|SetIsOpen false))
    (bind _opendoor (Timeline|OpenDoor Reverse)
      (:Update
        (Transformation|SetRelativeLocation (Variables|Default|GetDoor) (Math|Vector|MakeVector 0.0 (Math|Float|Lerp 0.0 2.6e+02 _opendoor) 0.0) false false))
      (:Finished
        (Utilities|Time|SetTimerbyEvent (delegate Custom|TryCloseDoor) 1.0 _output_get)))))

(fn ConstructionScript)