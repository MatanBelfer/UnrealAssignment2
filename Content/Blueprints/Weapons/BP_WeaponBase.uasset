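; BP_WeaponBase is a weapon base Blueprint whose only working logic is a Fire function that launches physical bullets.
; While the clip has ammo, Fire spawns BulletClass at the Muzzle, decrements ammo, passes gun and Holder to the bullet and impulses its Cone forward.
; It then plays a sound, located at the Muzzle's forward vector rather than its position, and refreshes player 0's HUD.
; An empty clip only prints a message.
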(event EventBeginPlay)

(event Collision|EventActorBeginOverlap
  (params (OtherActor :type Actor%20Object%20Reference)))

(event EventTick
  (params (DeltaSeconds :type Float%20%28single-precision%29)))

(fn ConstructionScript)

(fn Fire
  (bind _muzzle (Variables|Default|GetMuzzle))
  (bind _muzzle_2 (Variables|Default|GetMuzzle))
  (bind _returnvalue (Math|Vector|GetForwardVector _muzzle_2))
  (bind _returnvalue_2 (Transformation|GetWorldTransform _muzzle))
  (if (> (Variables|Default|GetAmmoInClip) 0.0)
    (bind _returnvalue_3 (Game|SpawnActorfromClass (Variables|Default|GetBulletClass) (Math|Transform|MakeTransform (.location _returnvalue_2) (.rotation _returnvalue_2) "0.100000,0.100000,0.100000") "AlwaysSpawn" "OverrideRootScale" 0 0))
    (bind _result (Math|Integer|DecrementInt (Variables|Default|GetAmmoInClip))
      (:%20%20
        (Variables|Default|SetAmmoInClip _result)
        (Variables|/Game/Blueprints/Weapons/BP_Bullet.BP_Bullet_C|SetGun _returnvalue_3 self)
        (Variables|/Game/Blueprints/Weapons/BP_Bullet.BP_Bullet_C|SetShooter _returnvalue_3 (Variables|Default|GetHolder))
        (Physics|AddImpulse (Variables|/Game/Blueprints/Weapons/BP_Bullet.BP_Bullet_C|GetCone _returnvalue_3) (* _returnvalue 2e+03) "None" false)
        (Audio|PlaySoundatLocation (Variables|Default|GetSound) _returnvalue "0, 0, 0" 1.0 1.0 0.0 0 0 0 0)
        (bind _asbp_player_controller (Utilities|Casting|CastToBP_PlayerController (Game|GetPlayerController 0)))
        (Default|UpdateHUD _asbp_player_controller)))
    (else
      (Development|PrintString "No bullets!"))))