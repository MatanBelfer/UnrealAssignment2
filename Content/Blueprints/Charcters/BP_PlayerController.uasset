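; Player controller that routes Enhanced Input to BP_PlayerCharacter for look, move, fire, reload, weapon switching and interaction.
; BeginPlay caches the character, adds the input mapping context and creates the HUD, which UpdateHUD refreshes from the character.
; Weapon switching cycles the character's weapon array by modulo, showing only the current weapon, then updates the HUD.
; Interact runs a short, debug-drawn camera line trace and sends ClickMessage to BPI_Clickable actors.
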(event Input|EnhancedActionEvents|EnhancedInputActionIA_Move
  (params (ActionValue :type Vector%202D%20Structure) (ElapsedSeconds :type Float%20%28double-precision%29) (TriggeredSeconds :type Float%20%28double-precision%29) (InputAction :type Input%20Action%20Object%20Reference :default "/Game/Blueprints/Input/IA_Move.IA_Move"))
  (bind _returnvalue (Pawn|GetControlRotation :!class /Script/Engine.Controller))
  (Pawn|Input|AddMovementInput (Variables|Default|GetAs%20BP%20Player%20Character) (Math|Vector|GetForwardVector (Math|Rotator|MakeRotator 0.0 0.0 (.yaw (Pawn|GetControlRotation :!class /Script/Engine.Controller)))) (.x ActionValue) false)
  (Pawn|Input|AddMovementInput (Game|GetPlayerCharacter 0) (Math|Vector|GetRightVector (Math|Rotator|MakeRotator (.roll _returnvalue) 0.0 (.yaw _returnvalue))) (.y ActionValue) false))

(event Input|EnhancedActionEvents|EnhancedInputActionIA_Look
  (params (ActionValue :type Vector%202D%20Structure) (ElapsedSeconds :type Float%20%28double-precision%29) (TriggeredSeconds :type Float%20%28double-precision%29) (InputAction :type Input%20Action%20Object%20Reference :default "/Game/Blueprints/Input/IA_Look.IA_Look"))
  (bind _as_bp_player_character (Variables|Default|GetAs%20BP%20Player%20Character))
  (Pawn|Input|AddControllerYawInput _as_bp_player_character (.x ActionValue))
  (Pawn|Input|AddControllerPitchInput _as_bp_player_character (.y ActionValue)))

(event Input|EnhancedActionEvents|EnhancedInputActionIA_Fire
  (params (ActionValue :type Boolean) (ElapsedSeconds :type Float%20%28double-precision%29) (TriggeredSeconds :type Float%20%28double-precision%29) (InputAction :type Input%20Action%20Object%20Reference :default "/Game/Blueprints/Input/IA_Fire.IA_Fire"))
  (Default|Fire (Variables|Default|GetAs%20BP%20Player%20Character)))

(event Input|EnhancedActionEvents|EnhancedInputActionIA_SwitchWeapon
  (params (ActionValue :type Boolean) (ElapsedSeconds :type Float%20%28double-precision%29) (TriggeredSeconds :type Float%20%28double-precision%29) (InputAction :type Input%20Action%20Object%20Reference :default "/Game/Blueprints/Input/IA_SwitchWeapon.IA_SwitchWeapon"))
  (CallFunction|SwitchWeapon))

(event Input|EnhancedActionEvents|EnhancedInputActionIA_Reload
  (params (ActionValue :type Boolean) (ElapsedSeconds :type Float%20%28double-precision%29) (TriggeredSeconds :type Float%20%28double-precision%29) (InputAction :type Input%20Action%20Object%20Reference :default "/Game/Blueprints/Input/IA_Reload.IA_Reload"))
  (Default|Reload (Variables|Default|GetAs%20BP%20Player%20Character)))

(event Input|EnhancedActionEvents|EnhancedInputActionIA_Interact
  (params (ActionValue :type Boolean) (ElapsedSeconds :type Float%20%28double-precision%29) (TriggeredSeconds :type Float%20%28double-precision%29) (InputAction :type Input%20Action%20Object%20Reference :default "/Game/Blueprints/Input/IA_Interact.IA_Interact"))
  (bind _as_bp_player_character (Variables|Default|GetAs%20BP%20Player%20Character))
  (bind _camera (Variables|/Game/Blueprints/Charcters/BP_PlayerCharacter.BP_PlayerCharacter_C|GetCamera _as_bp_player_character))
  (bind _returnvalue (Transformation|GetWorldLocation _camera))
  (bind _outhit (Collision|LineTraceByChannel _returnvalue (+ _returnvalue (* (Math|Vector|GetForwardVector _camera) 2.5e+02)) "TraceTypeQuery1" false (Utilities|Array|MakeArray (Variables|Default|GetAs%20BP%20Player%20Character)) "Persistent"))
  (if (Utilities|DoesObjectImplementInterface (.HitActor (Collision|BreakHitResult _outhit)) "/Game/Blueprints/Interfaces/BPI_Clickable.BPI_Clickable_C")
    (Class|BPIClickable|Click(Message) (.HitActor (Collision|BreakHitResult _outhit)) (.HitComponent (Collision|BreakHitResult _outhit)) (Variables|Default|GetAs%20BP%20Player%20Character))))

(event EventBeginPlay
  (bind _asbp_player_character (Utilities|Casting|CastToBP_PlayerCharacter (Game|GetPlayerCharacter 0))
    (:then
      (Variables|Default|SetAs%20BP%20Player%20Character _asbp_player_character)
      (Input|AddMappingContext (PlayerController|LocalPlayerSubsystems|GetEnhancedInputLocalPlayerSubsystem) "/Game/Blueprints/Input/IMC_Player.IMC_Player" 0 "(bIgnoreAllPressedKeysUntilRelease=True,bForceImmediately=False,bNotifyUserSettings=False)")
      (bind _returnvalue (UserInterface|CreateWidget "/Game/Blueprints/UI/HUD.HUD_C"))
      (bind _output_get (Variables|Default|SetHUD _returnvalue))
      (UserInterface|Viewport|AddtoViewport _output_get 0))
    (:CastFailed
      (Development|PrintString "Error finding player "))))

(fn ConstructionScript)

(fn UpdateHUD
  (bind _asbp_player_character (Utilities|Casting|CastToBP_PlayerCharacter (Game|GetPlayerCharacter 0)))
  (Default|UpdatePlayerHUD (Variables|Default|GetHUD) _asbp_player_character))

(fn SwitchWeapon
  (bind _as_bp_player_character (Variables|Default|GetAs%20BP%20Player%20Character))
  (bind _weaponarray (Variables|/Game/Blueprints/Charcters/BP_PlayerCharacter.BP_PlayerCharacter_C|GetWeaponArray _as_bp_player_character))
  (bind _returnvalue (Utilities|Array|Length _weaponarray))
  (if (> _returnvalue 1)
    (bind _result (Math|Integer|IncrementInt (Variables|/Game/Blueprints/Charcters/BP_PlayerCharacter.BP_PlayerCharacter_C|GetCurrentWeaponIndex (Variables|Default|GetAs%20BP%20Player%20Character)))
      (:%20%20
        (for (_array_element _array_index) (Variables|/Game/Blueprints/Charcters/BP_PlayerCharacter.BP_PlayerCharacter_C|GetWeaponArray (Variables|Default|GetAs%20BP%20Player%20Character))
          (if (== (Math|Integer|%(Integer) _result _returnvalue) _array_index)
            (Rendering|SetActorHiddenInGame _array_element false)
            (Variables|/Game/Blueprints/Charcters/BP_PlayerCharacter.BP_PlayerCharacter_C|SetCurrentWeapon (Variables|Default|GetAs%20BP%20Player%20Character) _array_element)
            (else
              (Rendering|SetActorHiddenInGame _array_element true))))
        (CallFunction|UpdateHUD)))))