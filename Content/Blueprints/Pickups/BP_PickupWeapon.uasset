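; Weapon pickup that offers a randomly chosen weapon from its pool.
; On BeginPlay it spawns a random class from PoolOfWeapons at the sphere collider, attaches it as the pickup object and removes the preview cube.
; It then creates a dynamic glow material and tints it by the weapon class's default ammo type, distinguishing rifles from pistols.
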(event EventBeginPlay
  (bind _sphere_collider (Variables|Default|GetSphere_Collider))
  (bind _glowmesh (Variables|Default|GetGlowMesh))
  (bind _returnvalue (Transformation|GetWorldTransform _sphere_collider))
  (|CallParentFunction)
  (Variables|Default|SetPickupType "NewEnumerator0")
  (bind _output_get (Variables|Default|SetWeaponClass (.OutItem (Utilities|Array|Random (Variables|Default|GetPoolOfWeapons)))))
  (bind _returnvalue_2 (Game|SpawnActorfromClass _output_get (Math|Transform|MakeTransform (.location _returnvalue) (.rotation _returnvalue) "1.000000,1.000000,1.000000") "AlwaysSpawn" "MultiplyWithRoot" 0 (.AmmoType (Utilities|GetClassDefaults _output_get)) 0))
  (bind _output_get_2 (Variables|Default|SetPickupObject _returnvalue_2))
  (Transformation|AttachActorToActor _output_get_2 self "None" "SnapToTarget" "SnapToTarget" "KeepRelative" true)
  (Components|DestroyComponent (Variables|Default|GetPreviewCube))
  (bind _returnvalue_3 (Rendering|Material|CreateDynamicMaterialInstance _glowmesh 0 (Rendering|Material|GetMaterial _glowmesh 0) "None" :!class /Script/Engine.PrimitiveComponent))
  (switch Utilities|FlowControl|Switch|SwitchonWeapon_Ammo_Type (.AmmoType (Utilities|GetClassDefaults (Variables|Default|GetWeaponClass)))
    (:NewEnumerator0
      (Rendering|Material|SetVectorParameterValue _returnvalue_3 "GlowColor" (Utilities|Struct|MakeLinearColor 1.0 1.0 1.0 1.0) :!class /Script/Engine.MaterialInstanceDynamic))
    (:NewEnumerator1
      (Rendering|Material|SetVectorParameterValue _returnvalue_3 "GlowColor" (Utilities|Struct|MakeLinearColor 1.0 0.0 0.0 1.0) :!class /Script/Engine.MaterialInstanceDynamic))))

(fn ConstructionScript
  (|CallParentFunction))