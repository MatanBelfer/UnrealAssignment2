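; Base pickup actor that floats and spins in the world and notifies the player on overlap.
; Tick offsets it vertically from its BeginPlay location with a degree-based sine wave, with FloatSpeed driving both the bob and yaw spin.
; Overlap with an actor tagged Player sets IsPickedup and sends OnPickupMessage to that actor with itself and PickupObject.
; The pickup neither hides nor destroys itself here.
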(event EventBeginPlay
  (Variables|Default|SetStartVector (Transformation|GetActorLocation)))

(event Collision|EventActorBeginOverlap
  (params (OtherActor :type Actor%20Object%20Reference))
  (if (Actor|ActorHasTag OtherActor "Player")
    (Variables|Default|SetIsPickedup true)
    (Class|BPIInteractable|OnPickup(Message) OtherActor self (Variables|Default|GetPickupObject))))

(event EventTick
  (params (DeltaSeconds :type Float%20%28single-precision%29))
  (bind _floatspeed (Variables|Default|GetFloatSpeed))
  (bind _returnvalue (* DeltaSeconds _floatspeed))
  (bind _output_get (Variables|Default|SetRunningTime%20 (+ _returnvalue (Variables|Default|GetRunningTime%20))))
  (Transformation|SetActorLocation (+ (Math|Vector|MakeVector 0.0 0.0 (* (Math|Trig|Sin(Degrees) _output_get) (Variables|Default|GetFloatAmplitude))) (Variables|Default|GetStartVector)) false false)
  (Transformation|AddActorLocalRotation (Math|Rotator|MakeRotator 0.0 0.0 _returnvalue) false false))

(fn ConstructionScript)