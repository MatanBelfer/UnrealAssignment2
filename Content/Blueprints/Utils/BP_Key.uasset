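; BP_Key is a numbered key button actor, likely part of a keypad, with a key mesh and a text label.
; Clicking it plays a click sound at the key's location and fires an OnButtonPressed dispatcher carrying its number.
; SetNumber stores the number and updates the label text, while Reset and the construction script are empty.
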(event EventBeginPlay)

(event EventClick
  (params (HitComponent :type Primitive%20Component%20Object%20Reference) (InstigatorActor :type Actor%20Object%20Reference))
  (Audio|PlaySoundatLocation "/Engine/VREditor/Sounds/UI/Click_on_Button.Click_on_Button" (Transformation|GetWorldLocation (Variables|Default|GetKey)) "0, 0, 0" 1.0 1.0 0.0 0 0 0 0)
  (Default|CallOnButtonPressed (Variables|Default|GetNumber)))

(fn ConstructionScript)

(fn Reset)

(fn SetNumber
  (params (KeyNumber :type Integer))
  (bind _output_get (Variables|Default|SetNumber KeyNumber))
  (Rendering|Components|TextRender|SetText (Variables|Default|GetTXT_BTN) (Utilities|Text|ToText(Integer) _output_get)))