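; BP_GameMode tracks the player and enemies to decide the win or loss of a match.
; On BeginPlay it caches the player character and every BP_EnemyCharcter in the level.
; OnDied prints a loss message and changes the state of all remaining enemies when the player dies.
; Otherwise it removes the dead enemy from the list and prints a win message once the list is empty.
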(event Custom|OnDied
  (params (Actor :type BP%20Charcter%20Base%20Object%20Reference))
  (Utilities|Casting|CastToBP_PlayerCharacter Actor
    (:then
      (Development|PrintString "You Lost!" true true "(R=1.000000,G=0.058219,B=0.120818,A=1.000000)" 3e+01)
      (for _array_element (Variables|Default|GetEnemies)
        (Default|ChangeState _array_element "NewEnumerator0")))
    (:CastFailed
      (bind _asbp_enemy_charcter (Utilities|Casting|CastToBP_EnemyCharcter Actor))
      (bind _returnvalue (Utilities|Array|RemoveItem (Variables|Default|GetEnemies) _asbp_enemy_charcter))
      (if _returnvalue
        (if (== (Utilities|Array|Length (Variables|Default|GetEnemies)) 0)
          (Development|PrintString "Win"))))))

(event EventBeginPlay
  (bind _asbp_player_character (Utilities|Casting|CastToBP_PlayerCharacter (Game|GetPlayerCharacter 0)))
  (Variables|Default|SetPlayer _asbp_player_character)
  (bind _outactors (Actor|GetAllActorsOfClass "/Game/Blueprints/Charcters/BP_EnemyCharcter.BP_EnemyCharcter_C"))
  (Variables|Default|SetEnemies _outactors))

(fn ConstructionScript)