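; Random pickup actor that turns into a weapon or ammo pickup when play begins.
; BeginPlay picks a random pickup type, then a random class from the matching pool, spawning it at the sphere collider, attaching it and destroying the preview cube.
; The class default AmmoType sets the GlowMesh color through a dynamic material instance, distinguishing rifle from pistol.
; This graph contains no active overlap or tick logic.
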(event EventBeginPlay
  (bind _sphere_collider (Variables|Default|GetSphere_Collider))
  (bind _sphere_collider_2 (Variables|Default|GetSphere_Collider))
  (bind _pickuptypearray (Variables|Default|GetPickupTypeArray))
  (bind _glowmesh (Variables|Default|GetGlowMesh))
  (bind _returnvalue (Transformation|GetWorldTransform _sphere_collider))
  (bind _returnvalue_2 (Transformation|GetWorldTransform _sphere_collider_2))
  (|CallParentFunction)
  (bind _enumvalue (|ForEachPickup_Type)
    (:LoopBody
      (Utilities|Array|Add _pickuptypearray _enumvalue))
    (:then
      (bind _output_get (Variables|Default|SetPickupType (.OutItem (Utilities|Array|Random _pickuptypearray))))
      (switch Utilities|FlowControl|Switch|SwitchonPickup_Type _output_get
        (:NewEnumerator0
          (bind _output_get_2 (Variables|Default|SetWeaponClass (.OutItem (Utilities|Array|Random (Variables|Default|GetPoolOfWeapons)))))
          (Variables|Default|SetAmmo%20Type (.AmmoType (Utilities|GetClassDefaults _output_get_2)))
          (bind _returnvalue_3 (Game|SpawnActorfromClass _output_get_2 (Math|Transform|MakeTransform (.location _returnvalue_2) (.rotation _returnvalue_2) "1.000000,1.000000,1.000000") "AlwaysSpawn" "MultiplyWithRoot" 0 (.AmmoType (Utilities|GetClassDefaults _output_get_2)) 0))
          (bind _output_get_3 (Variables|Default|SetPickupObject _returnvalue_3))
          (Transformation|AttachActorToActor _output_get_3 self "None" "SnapToTarget" "SnapToTarget" "KeepRelative" true)
          (Components|DestroyComponent (Variables|Default|GetPreviewCube)))
        (:NewEnumerator1
          (bind _output_get_4 (Variables|Default|SetAmmoClass (.OutItem (Utilities|Array|Random (Variables|Default|GetPoolOfAmmo)))))
          (Variables|Default|SetAmmo%20Type (.AmmoType (Utilities|GetClassDefaults _output_get_4)))
          (bind _returnvalue_4 (Game|SpawnActorfromClass _output_get_4 (Math|Transform|MakeTransform (.location _returnvalue) (.rotation _returnvalue) "1.000000,1.000000,1.000000") "AlwaysSpawn" "MultiplyWithRoot" 0 (.AmmoType (Utilities|GetClassDefaults _output_get_4)) 0))
          (bind _output_get_5 (Variables|Default|SetPickupObject _returnvalue_4))
          (Transformation|AttachActorToActor _output_get_5 self "None" "SnapToTarget" "SnapToTarget" "KeepRelative" true)
          (Components|DestroyComponent (Variables|Default|GetPreviewCube))))
      (bind _returnvalue_5 (Rendering|Material|CreateDynamicMaterialInstance _glowmesh 0 (Rendering|Material|GetMaterial _glowmesh 0) "None" :!class /Script/Engine.PrimitiveComponent))
      (switch Utilities|FlowControl|Switch|SwitchonWeapon_Ammo_Type (Variables|Default|GetAmmo%20Type)
        (:NewEnumerator0
          (Rendering|Material|SetVectorParameterValue _returnvalue_5 "GlowColor" (Utilities|Struct|MakeLinearColor 1.0 1.0 1.0 1.0) :!class /Script/Engine.MaterialInstanceDynamic))
        (:NewEnumerator1
          (Rendering|Material|SetVectorParameterValue _returnvalue_5 "GlowColor" (Utilities|Struct|MakeLinearColor 1.0 0.0 0.0 1.0) :!class /Script/Engine.MaterialInstanceDynamic))))))

(event Collision|EventActorBeginOverlap
  (params (OtherActor :type Actor%20Object%20Reference))
  (|CallParentFunction OtherActor) ; This node is disabled and will not be called.\nDrag off pins to build functionality.
)

(event EventTick
  (params (DeltaSeconds :type Float%20%28single-precision%29))
  (|CallParentFunction DeltaSeconds) ; This node is disabled and will not be called.\nDrag off pins to build functionality.
)

(fn ConstructionScript
  (|CallParentFunction))